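; Paper2D player character that runs, jumps, shoots BP_Shot projectiles and takes damage, with a HUD widget created on BeginPlay.
; Input and events set boolean flags, which a priority chain of check macros resolves into a state each Tick.
; That state selects the sprite's flipbook from the FlipBooks array.
; Damage disables input and either kills or knocks back with a blinking sprite, restoring control shortly after landing.
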(event `self.ReceiveAnyDamage`
  (params (Damage :type "Float (single-precision)") (DamageType :type "DamageType Object Reference") (InstigatedBy :type "Controller Object Reference") (DamageCauser :type "Actor Object Reference"))
  ;[1 1 1] DamageSystem
  (set `self.IsHit` true)
  (`self.DisableInput` (`GameplayStatics.GetPlayerController` 0))
  (bind _output_get (set `self.HealthCurrent` (- (`self.HealthCurrent`) Damage)))
  (if (<= _output_get 0.0)
    (set `self.IsDead` true)
    (`self.DisableInput` (`GameplayStatics.GetPlayerController` 0))
    (else
      (`CharacterMovementComponent.AddImpulse` (`self.CharacterMovement`) (`KismetMathLibrary.MakeVector` (* (`self.Facing`) (`self.KnockBack`)) 0.0 40000.0) false)
      (`KismetSystemLibrary.K2_SetTimer` null "Blink" 0.1 true)
      (`KismetSystemLibrary.Delay` 1.0)
      (`KismetSystemLibrary.K2_ClearTimer` null "Blink")
      (`SceneComponent.SetVisibility` (`self.Sprite`) true false))))

(event `Blink`
  ;[1 1 1] DamageSystem
  (`SceneComponent.ToggleVisibility` (`self.Sprite`) false))

(event `self.ReceiveBeginPlay`
  ;[1 1 1] Initialize
  (`|ExecutionSequence`
    (:`then_0`
      (`ActorComponent.SetIsReplicated` (`self.Sprite`) true))
    (:`then_1`
      (bind _returnvalue (`|CreateWidget` "/Game/Paper2DTuto/Blueprint/Widget_HUD.Widget_HUD_C" (`GameplayStatics.GetPlayerController` 0)))
      (bind _output_get (set `self.HealthBar` _returnvalue))
      (`UserWidget.AddToViewport` _output_get 0))))

(event `UpdateAnimation`
  ;[1 1 1] Update Animation
  (bind _stateflipbook (`self.GetStateFlipbook` (`self.State`)))
  (`PaperFlipbookComponent.SetFlipbook` (`self.Sprite`) _stateflipbook))

(event `InputAxis|MoveRight`
  (params (AxisValue :type "Float (single-precision)"))
  ;[1 1 1] Handle movement
  (`self.AddMovementInput` (1.0 0.0 0.0) AxisValue)
  (`/Engine/EditorBlueprintResources/StandardMacros.CompareFloat` AxisValue
    (:`>`
      (`Controller.SetControlRotation` (`self.GetController`) (`KismetMathLibrary.MakeRot` 0.0 0.0))
      (set `self.Facing` -1)
      (set `self.IsRunning` true :!label _label))
    (:`==`
      (set `self.IsRunning` false))
    (:`<`
      (`Controller.SetControlRotation` (`self.GetController`) (`KismetMathLibrary.MakeRot` 0.0 180.0))
      (set `self.Facing` 1)
      (goto _label))))

(event `self.ReceiveTick`
  (params (DeltaSeconds :type "Float (single-precision)"))
  ;[1 1 1] Update Animation
  (`self.StateMachine`)
  (`self.UpdateAnimation`))

(event `InputAction|Jump`
  ;[1 1 1] Handle Jump
  (:`Pressed`
    (`self.Jump` :!label _label_2)
    (set `self.IsJumping` true))
  (:`Released`
    (`self.StopJumping` :!label _label_3)))

(event `InputTouch`
  (params (Location :type "Vector Structure") (FingerIndex :type "ETouchIndex Enum"))
  ;[1 1 1] Handle Jump
  (:`Pressed`
    (goto _label_2))
  (:`Released`
    (goto _label_3)))

(event `self.OnLanded`
  (params (Hit :type "HitResult Structure (by ref)"))
  ;[1 1 1] Handle Jump
  (set `self.IsLanding` true)
  (if (`self.IsHit`)
    (`KismetSystemLibrary.Delay` 0.2)
    (`self.EnableInput` (`GameplayStatics.GetPlayerController` 0))
    (set `self.IsHit` false))
  (set `self.IsLanding` false)
  (set `self.IsJumping` false))

(event `InputAction|Shoot`
  ;[1 1 1] Handle Shoot
  (:`Pressed`
    (`|SpawnActorFromClass` "/Game/Paper2DTuto/Blueprint/BP_Shot.BP_Shot_C" (`SceneComponent.K2_GetComponentToWorld` (`self.Arrow1`)) true)
    (set `self.IsShooting` true))
  (:`Released`
    (`KismetSystemLibrary.RetriggerableDelay` 0.3)
    (set `self.IsShooting` false)))

(fn `GetStateFlipbook`
  (params (State :type "/Game/Paper2DTuto/Blueprint/Char_States Enum"))
  (returns (StateFlipbook :type "PaperFlipbook Object Reference"))
  (for _array_element (`self.FlipBooks`)
    (if (`|EnumEquality` (break `/Game/Paper2DTuto/Blueprint/S_States` _array_element) State)
      (break)))
  (return (`.FlipBook_5_BE9F1BB740262B3973306C8D3EB054F6` (break `/Game/Paper2DTuto/Blueprint/S_States` _array_element))))

(fn `StateMachine`
  (returns (State :type "/Game/Paper2DTuto/Blueprint/Char_States Enum"))
  (if (`self.IsDead`)
    (set `self.State` "NewEnumerator5")
    (elif (`self.IsLanding`)
      (if (`self.IsHit`)
        (set `self.State` "NewEnumerator6")
        (else
          (if (`self.IsHit`) :!label _label
            (set `self.State` "NewEnumerator4")
            (elif (`self.IsShooting`)
              (if (`self.IsJumping`)
                (set `self.State` "NewEnumerator9")
                (else
                  (if (`self.IsShooting`) :!label _label_2
                    (if (`self.IsRunning`)
                      (set `self.State` "NewEnumerator8")
                      (else
                        (if (`self.IsShooting`) :!label _label_3
                          (set `self.State` "NewEnumerator7")
                          (elif (`self.IsJumping`)
                            (set `self.State` "NewEnumerator2")
                            (elif (`self.IsRunning`)
                              (set `self.State` "NewEnumerator1")
                              (else
                                (set `self.State` "NewEnumerator0")))))))
                    (else
                      (goto _label_3)))))
              (else
                (goto _label_2))))))
      (else
        (goto _label))))
  (return (`self.State`)))

(fn `UserConstructionScript`)